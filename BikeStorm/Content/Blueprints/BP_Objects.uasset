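; BP_Objects is a short-lived physics prop with a random mesh that is pushed by a constant force every tick and destroyed after 20 seconds.
; On BeginPlay a coin flip decides whether the force direction aims at the player's starting position or keeps its default.
; The construction script maps Meshes to Weights for mass overrides, but separate random picks can mismatch mesh and mass or index past the array.
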(event `self.ReceiveTick`
  (params (DeltaSeconds :type "Float (single-precision)"))
  (`PrimitiveComponent.AddForce` (`self.StaticMesh`) (* (`self.DirectionToPlayer`) (`self.Force`)) "None" false))

(event `Destroy`
  (`self.K2_DestroyActor`))

(event `self.ReceiveBeginPlay`
  (bind _staticmesh (`self.StaticMesh`))
  (bind _meshes (`self.Meshes`))
  (bind _output (`|GetArrayItem` _meshes (`KismetMathLibrary.RandomIntegerInRange` 0 (`KismetArrayLibrary.Array_Length` _meshes))))
  (bind (_value _returnvalue) (`BlueprintMapLibrary.Map_Find` (`self.Objects`) _output))
  (`|ExecutionSequence`
    (:`then_0`
      (`KismetSystemLibrary.K2_SetTimerDelegate` (delegate `Destroy`) 20.0))
    (:`then_1`
      (bind _asbp_player_character (cast `/Game/Blueprints/BP_PlayerCharacter` (`GameplayStatics.GetPlayerCharacter` 0)))
      (set `self.PlayerReference` _asbp_player_character)
      (if (== (`KismetMathLibrary.RandomIntegerInRange` 0 1) 1)
        (set `self.DirectionToPlayer` (`KismetMathLibrary.GetDirectionUnitVector` (`SceneComponent.K2_GetComponentLocation` (`self.StaticMesh`)) (`self.K2_GetActorLocation` (`self.PlayerReference`))))))
    (:`then_2`
      (if _returnvalue
        (`StaticMeshComponent.SetStaticMesh` _staticmesh _output)
        (`PrimitiveComponent.SetMassOverrideInKg` _staticmesh "None" _value true)
        (`SceneComponent.K2_SetRelativeRotation` _staticmesh (`KismetMathLibrary.RandomRotator` false) false false)))))

(fn `UserConstructionScript`
  (for (_array_element _array_index) (`self.Meshes`)
    (`BlueprintMapLibrary.Map_Add` (`self.Objects`) _array_element (`|GetArrayItem` (`self.Weights`) _array_index))))