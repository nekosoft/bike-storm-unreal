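; Game mode that shows the HUD and repeatedly spawns BP_Objects actors at a fixed Y offset from the player, at random heights.
; BeginPlay adds the HUD widget and starts a looping timer with a random interval based on SpawnTime, while each spawn increments NumSpawned.
; Tick periodically lowers SpawnTime, but the timer's interval is set only once, so the running spawn rate stays unchanged.
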(event `self.ReceiveBeginPlay`
  (bind _spawntime (`self.SpawnTime`))
  (`|ExecutionSequence`
    (:`then_0`
      (bind _returnvalue (`|CreateWidget` "/Game/Blueprints/BP_HUD.BP_HUD_C"))
      (bind _output_get (set `self.HUDReference` _returnvalue))
      (`UserWidget.AddToViewport` _output_get 0))
    (:`then_1`
      (`KismetSystemLibrary.K2_SetTimerDelegate` (delegate `SpawnObject`) (`KismetMathLibrary.RandomFloatInRange` _spawntime (* _spawntime 2.0)) true))))

(event `SpawnObject`
  (bind (_returnvalue_x _returnvalue_y) (`KismetMathLibrary.BreakVector` (`SceneComponent.K2_GetComponentLocation` (`Character.CapsuleComponent` (`GameplayStatics.GetPlayerCharacter` 0)))))
  (`|SpawnActorFromClass` "/Game/Blueprints/BP_Objects.BP_Objects_C" (`KismetMathLibrary.MakeTransform` (`KismetMathLibrary.MakeVector` 0.0 (+ _returnvalue_y -1500.0) (`KismetMathLibrary.RandomFloatInRange` 0.0 500.0)) (struct :`Yaw` 90.0) (0.75 0.75 0.75)) "Undefined" "OverrideRootScale" null null)
  (`/Engine/EditorBlueprintResources/StandardMacros.IncrementInt` (`self.NumSpawned`)))

(event `self.ReceiveTick`
  (params (DeltaSeconds :type "Float (single-precision)"))
  (bind _timepassed (`self.TimePassed`))
  (bind _spawntime (`self.SpawnTime`))
  (if (> _timepassed (`self.TimeThreshHold`))
    (set `self.TimePassed` 0.0)
    (if (> _spawntime 0.0)
      (set `self.SpawnTime` (- _spawntime 0.2)))
    (else
      (set `self.TimePassed` (+ DeltaSeconds _timepassed)))))

(fn `UserConstructionScript`)